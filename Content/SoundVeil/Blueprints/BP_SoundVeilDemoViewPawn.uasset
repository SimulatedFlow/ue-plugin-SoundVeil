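; Demo view pawn for SoundVeil that provides keyboard controls for testing the system in a level.
; Tab toggles cursor mode, while mouse-based traces let C place or remove curtains, R rotate them and X toggle a hit actor's audio.
; F3 registers or unregisters SoundVeil components on stress-tagged demo sources.
; PageUp and PageDown switch audible-tagged sources between boosted and normal volume.
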(event Input|KeyboardEvents|Tab
  (params (Key :type Key%20Structure))
  (bind _returnvalue (Game|GetPlayerController 0))
  (:Pressed
    (if (Variables|Default|GetbCursorMode)
      (Input|SetInputModeGameOnly _returnvalue false)
      (Variables|/Script/Engine.PlayerController|SetbShowMouseCursor _returnvalue false)
      (Variables|Default|SetbCursorMode false)
      (else
        (Input|SetInputModeGameandUI _returnvalue 0 "DoNotLock" true false)
        (Variables|/Script/Engine.PlayerController|SetbShowMouseCursor _returnvalue true)
        (Variables|Default|SetbCursorMode true)))))

(event Input|KeyboardEvents|F3
  (params (Key :type Key%20Structure))
  (:Pressed
    (Variables|Default|SetbStressOn (not (Variables|Default|GetbStressOn)))
    (bind _outactors (Actor|GetAllActorsOfClasswithTag "/SoundVeil/SoundVeil/Blueprints/BP_SoundVeilDemoSource.BP_SoundVeilDemoSource_C" "SoundVeilStress"))
    (for _array_element _outactors
      (bind _assoundveil_source (Utilities|Casting|CastToSoundVeilComponent (Actor|GetComponentbyClass _array_element "/Script/SoundVeil.SoundVeilComponent")))
      (if (Variables|Default|GetbStressOn)
        (Class|SoundVeilComponent|Register _assoundveil_source)
        (else
          (Class|SoundVeilComponent|Unregister _assoundveil_source))))))

(event Input|KeyboardEvents|X
  (params (Key :type Key%20Structure))
  (bind _returnvalue (Game|GetPlayerController 0))
  (bind (_worldlocation _worlddirection) (Game|Player|ConvertMouseLocationToWorldSpace _returnvalue))
  (:Pressed
    (bind (_outhit _returnvalue_2) (Collision|LineTraceByChannel _worldlocation (+ _worldlocation (* _worlddirection "(X=12000.000000,Y=12000.000000,Z=12000.000000)")) "TraceTypeQuery1" false 0 "None"))
    (if _returnvalue_2
      (Components|Activation|ToggleActive (Actor|GetComponentbyClass (.HitActor (Collision|BreakHitResult _outhit)) "/Script/Engine.AudioComponent")))))

(event Input|KeyboardEvents|C
  (params (Key :type Key%20Structure))
  (bind _returnvalue (Game|GetPlayerController 0))
  (bind (_worldlocation _worlddirection) (Game|Player|ConvertMouseLocationToWorldSpace _returnvalue))
  (:Pressed
    (bind (_outhit _returnvalue_2) (Collision|LineTraceByChannel _worldlocation (+ _worldlocation (* _worlddirection "(X=12000.000000,Y=12000.000000,Z=12000.000000)")) "TraceTypeQuery1" false 0 "None"))
    (if _returnvalue_2
      (if (Actor|ActorHasTag (.HitActor (Collision|BreakHitResult _outhit)) "SoundVeilCurtain")
        (Actor|DestroyActor (.HitActor (Collision|BreakHitResult _outhit)))
        (else
          (Game|SpawnActorfromClass "/SoundVeil/SoundVeil/Blueprints/BP_SoundVeilDemoCurtain.BP_SoundVeilDemoCurtain_C" (Math|Transform|MakeTransform (.Location (Collision|BreakHitResult _outhit))) "AlwaysSpawn" "MultiplyWithRoot" 0 0))))))

(event Input|KeyboardEvents|PageUp
  (params (Key :type Key%20Structure))
  (:Pressed
    (bind _outactors (Actor|GetAllActorsOfClasswithTag "/SoundVeil/SoundVeil/Blueprints/BP_SoundVeilDemoSource.BP_SoundVeilDemoSource_C" "SoundVeilAudible"))
    (for _array_element _outactors
      (bind _asaudio_component (Utilities|Casting|CastToAudioComponent (Actor|GetComponentbyClass _array_element "/Script/Engine.AudioComponent")))
      (Audio|Components|Audio|AdjustVolume _asaudio_component 0.1 3.0 "Linear" :!class /Script/Engine.AudioComponent))))

(event Input|KeyboardEvents|PageDown
  (params (Key :type Key%20Structure))
  (:Pressed
    (bind _outactors (Actor|GetAllActorsOfClasswithTag "/SoundVeil/SoundVeil/Blueprints/BP_SoundVeilDemoSource.BP_SoundVeilDemoSource_C" "SoundVeilAudible"))
    (for _array_element _outactors
      (bind _asaudio_component (Utilities|Casting|CastToAudioComponent (Actor|GetComponentbyClass _array_element "/Script/Engine.AudioComponent")))
      (Audio|Components|Audio|AdjustVolume _asaudio_component 0.1 1.0 "Linear" :!class /Script/Engine.AudioComponent))))

(event Input|KeyboardEvents|R
  (params (Key :type Key%20Structure))
  (bind _returnvalue (Game|GetPlayerController 0))
  (bind (_hitresult _returnvalue_2) (Game|Player|GetHitResultUnderCursorbyChannel _returnvalue "TraceTypeQuery1" false))
  (bind _hitactor (Collision|BreakHitResult _hitresult))
  (:Pressed
    (if _returnvalue_2
      (if (Actor|ActorHasTag _hitactor "SoundVeilCurtain")
        (Class|Actor|AddActorWorldRotation _hitactor (Math|Rotator|MakeRotator 0.0 0.0 45.0))))))

(fn ConstructionScript)