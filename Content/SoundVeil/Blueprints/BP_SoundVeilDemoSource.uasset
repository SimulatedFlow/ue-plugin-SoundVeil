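; Demo sound emitter actor for SoundVeil that makes the occlusion of its audio visible.
; The construction script applies the exposed sound and volume to the Audio component and the wall profile to the Veil component.
; On BeginPlay it starts the audio at a random time offset into the sound.
; Veil occlusion changes drive an Occlusion scalar parameter on the Column's materials.
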(event OnOcclusionChanged(Veil)
  (params (Occlusion :type Float%20%28single-precision%29))
  (Rendering|Material|SetScalarParameterValueonMaterials (Variables|Default|GetColumn) "Occlusion" Occlusion))

(event EventBeginPlay
  (Audio|Components|Audio|Play (Variables|Default|GetAudio) (Math|Random|RandomFloatinRange 0.0 7.5)))

(event Collision|EventActorBeginOverlap
  (params (OtherActor :type Actor%20Object%20Reference)))

(event EventTick
  (params (DeltaSeconds :type Float%20%28single-precision%29)))

(fn ConstructionScript
  (bind _audio (Variables|Default|GetAudio))
  (Variables|/Script/Engine.AudioComponent|SetSound _audio (Variables|SoundVeilDemo|GetSourceSound))
  (Variables|/Script/Engine.AudioComponent|SetVolumeMultiplier _audio (Variables|SoundVeilDemo|GetSourceVolume))
  (Class|SoundVeilComponent|SetProfile (Variables|Default|GetVeil) (Variables|SoundVeilDemo|GetWallProfile)))