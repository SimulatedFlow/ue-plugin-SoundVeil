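; Sliding demo door for SoundVeil that opens and closes according to a DoorOpen flag.
; SetDoorOpen only sets the flag; the Blueprint has no trigger logic of its own.
; Every Tick, OpenAlpha eases toward open or closed with FInterpTo and offsets DoorMesh along local Y by SlideDistance, at a fixed relative height.
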(event EventBeginPlay)

(event Collision|EventActorBeginOverlap
  (params (OtherActor :type Actor%20Object%20Reference)))

(event EventTick
  (params (DeltaSeconds :type Float%20%28single-precision%29))
  (bind _slidespeed (Variables|Default|GetSlideSpeed))
  (if (Variables|Default|GetDoorOpen)
    (Variables|Default|SetOpenAlpha (Math|Interpolation|FInterpTo (Variables|Default|GetOpenAlpha) 1.0 DeltaSeconds _slidespeed))
    (else
      (Variables|Default|SetOpenAlpha (Math|Interpolation|FInterpTo (Variables|Default|GetOpenAlpha) 0.0 DeltaSeconds _slidespeed))))
  (Transformation|SetRelativeLocation (Variables|Default|GetDoorMesh) (Math|Vector|MakeVector 0.0 (* (Variables|Default|GetOpenAlpha) (Variables|Default|GetSlideDistance)) 1.5e+02) false false))

(fn ConstructionScript)

(fn SetDoorOpen
  (params (Open :type Boolean))
  (Variables|Default|SetDoorOpen Open))